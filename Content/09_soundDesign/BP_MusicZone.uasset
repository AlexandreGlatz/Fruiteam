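; BP_MusicZone is a trigger volume that switches from ambient music to a 2D enemy track when a Player-tagged actor enters.
; On entry it fades out the referenced ambient audio and spawns and fades in the new track.
; On any actor's exit it fades out that track, without a tag check and without restoring the ambient music.
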(event OnComponentBeginOverlap(trigger)
  (params (OverlappedComponent :type Primitive%20Component%20Object%20Reference) (OtherActor :type Actor%20Object%20Reference) (OtherComp :type Primitive%20Component%20Object%20Reference) (OtherBodyIndex :type Integer) (bFromSweep :type Boolean) (SweepResult :type Hit%20Result%20Structure%20%28by%20ref%29))
  (if (Actor|ActorHasTag OtherActor "Player")
    (Audio|Components|Audio|FadeOut (Actor|GetComponentbyClass (Variables|Default|GetAmbientmusic) "/Script/Engine.AudioComponent") 1.0 0.0 "Linear" :!class /Script/Engine.AudioComponent)
    (bind _returnvalue (Audio|SpawnSound2D "/Game/09_soundDesign/enemy.enemy" 0.5 1.0 0.0 0))
    (bind _output_get (Variables|Default|Setmusic _returnvalue))
    (Audio|Components|Audio|FadeIn _output_get 0.5 0.5 0.0 "Linear" :!class /Script/Engine.AudioComponent)))

(event OnComponentEndOverlap(trigger)
  (params (OverlappedComponent :type Primitive%20Component%20Object%20Reference) (OtherActor :type Actor%20Object%20Reference) (OtherComp :type Primitive%20Component%20Object%20Reference) (OtherBodyIndex :type Integer))
  (if true
    (bind _music (Variables|Default|Getmusic)
      (:then
        (Audio|Components|Audio|FadeOut _music 0.5 0.0 "Linear" :!class /Script/Engine.AudioComponent))
      (:else))))

(fn ConstructionScript)