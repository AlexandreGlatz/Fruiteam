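; Berry follower character that the player collects on entering its follow radius, with one of two skeletal meshes picked at random.
; Delegates leader, target and state changes to its AIC_Berry controller.
; Melee attacks deal damage and signal animation completion, or end the fight and player's strong power-up when the target is invalid.
; Jumps relay down the line with index-based delays, and death removes it from the player before destroying it.
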(event OnComponentBeginOverlap(followRadius)
  (params (OverlappedComponent :type Primitive%20Component%20Object%20Reference) (OtherActor :type Actor%20Object%20Reference) (OtherComp :type Primitive%20Component%20Object%20Reference) (OtherBodyIndex :type Integer) (bFromSweep :type Boolean) (SweepResult :type Hit%20Result%20Structure%20%28by%20ref%29))
  (bind _asbp_third_person_character (Utilities|Casting|CastToBP_ThirdPersonCharacter OtherActor))
  (Utilities|FlowControl|DoOnce false
    (:Completed
      (Default|TakeBerry _asbp_third_person_character self)
      (Default|SetState (.AsAIC%20Berry (Utilities|Casting|CastToAIC_Berry (Pawn|GetController))) "NewEnumerator0"))))

(event EventBeginPlay
  (bind _mesh (Variables|Character|GetMesh))
  (Utilities|FlowControl|Sequence
    (:then_0
      (Variables|Default|Sethealth (Variables|Default|GetmaxHealth))
      (Variables|Default|Setdamages (Variables|Default|GetbaseDamages)))
    (:then_1
      (if (< (Math|Random|RandomIntegerinRange 0 100) 50)
        (Components|SkeletalMesh|SetSkeletalMeshAsset _mesh "/Game/Characters/Anim_Walk.Anim_Walk")
        (else
          (Components|SkeletalMesh|SetSkeletalMeshAsset _mesh "/Game/Characters/Blue_Guy.Blue_Guy"))))))

(event Collision|EventActorBeginOverlap
  (params (OtherActor :type Actor%20Object%20Reference)))

(event EventTick
  (params (DeltaSeconds :type Float%20%28single-precision%29)))

(event Custom|OnJump
  (params (nextInLine :type BP%20Berry%20Object%20Reference) (index :type Integer))
  (Utilities|FlowControl|Sequence
    (:then_0
      (Variables|/Script/Engine.CharacterMovementComponent|SetbNotifyApex (Variables|Character|GetCharacterMovement) true)
      (Utilities|FlowControl|Delay (* index 0.2))
      (Utilities|IsValid nextInLine
        (:Is%20Valid
          (Character|Jump nextInLine))))
    (:then_1
      (Variables|Default|SetisJumping true)
      (Utilities|FlowControl|Delay 0.5)
      (Variables|Default|SetisJumping false))))

(event Custom|EndOfFight
  (Variables|Default|Setdamages (Variables|Default|GetbaseDamages))
  (Default|StopStrongPowerUp (.AsBP%20Third%20Person%20Character (Utilities|Casting|CastToBP_ThirdPersonCharacter (Game|GetPlayerCharacter 0)))))

(event EventMeleeAttack
  (params (targetToAttack :type Actor%20Object%20Reference))
  (bind _ac_finishattackanimation (Variables|Default|GetAC_FinishAttackAnimation))
  (Utilities|IsValid targetToAttack
    (:Is%20Valid
      (Class|BPIDamagable|TakeDamage(Message) targetToAttack (Variables|Default|Getdamages))
      (Variables|Default|SetisAttacking true)
      (Utilities|FlowControl|Delay 0.75)
      (Variables|Default|SetisAttacking false)
      (Class|BPIEvent|Notify(Message) _ac_finishattackanimation))
    (:Is%20Not%20Valid
      (Default|SetState (.AsAIC%20Berry (Utilities|Casting|CastToAIC_Berry (Pawn|GetController))) "NewEnumerator0")
      (CallFunction|EndOfFight)
      (Default|Notify _ac_finishattackanimation))))

(event EventTakeDamage
  (params (damages :type Integer))
  (Variables|Default|Sethealth (Math|Integer|Clamp(Integer) (- (Variables|Default|Gethealth) damages) 0 (Variables|Default|GetmaxHealth)))
  (if (<= (Math|Integer|Clamp(Integer) (- (Variables|Default|Gethealth) damages) 0 (Variables|Default|GetmaxHealth)) 0)
    (CallFunction|Die)))

(event EventDie
  (bind _asbp_third_person_character (Utilities|Casting|CastToBP_ThirdPersonCharacter (Game|GetPlayerCharacter 0)))
  (Default|RemoveBerry _asbp_third_person_character self)
  (Actor|DestroyActor))

(fn ConstructionScript)

(fn SetLeader
  (params (leader :type Actor%20Object%20Reference))
  (bind _output_get (Variables|Default|Setleader leader))
  (Default|SetLeader (.AsAIC%20Berry (Utilities|Casting|CastToAIC_Berry (Pawn|GetController))) _output_get))

(fn Attack
  (params (target :type Actor%20Object%20Reference))
  (bind _returnvalue (Pawn|GetController))
  (bind _asaic_berry (Utilities|Casting|CastToAIC_Berry _returnvalue))
  (Default|SetTarget _asaic_berry target)
  (Default|SetState _asaic_berry "NewEnumerator1"))

(fn GetIsDead
  (return false))