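; Boss enemy that fights the player through a damageable interface and drops berries on death.
; Entering its encounter radius calls AttackEnemy on the player and switches the AIC_Enemy controller's state.
; Melee attacks deal damage, then fire a finish notification after a delay.
; Damage updates a camera-facing health bar widget and triggers Die at zero, which spawns berries above the boss and destroys it.
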(event OnComponentBeginOverlap(EncounterRadius)
  (params (OverlappedComponent :type Primitive%20Component%20Object%20Reference) (OtherActor :type Actor%20Object%20Reference) (OtherComp :type Primitive%20Component%20Object%20Reference) (OtherBodyIndex :type Integer) (bFromSweep :type Boolean) (SweepResult :type Hit%20Result%20Structure%20%28by%20ref%29))
  (bind _asbp_third_person_character (Utilities|Casting|CastToBP_ThirdPersonCharacter OtherActor))
  (Default|AttackEnemy _asbp_third_person_character self)
  (Default|SetState (.AsAIC%20Enemy (Utilities|Casting|CastToAIC_Enemy (Pawn|GetController))) "NewEnumerator1"))

(event EventBeginPlay
  (Variables|Default|Sethealth (Variables|Default|GetmaxHealth)))

(event Collision|EventActorBeginOverlap
  (params (OtherActor :type Actor%20Object%20Reference)))

(event EventTick
  (params (DeltaSeconds :type Float%20%28single-precision%29))
  (bind _widget (Variables|Default|GetWidget))
  (Transformation|SetWorldRotation _widget (Math|Rotator|FindLookatRotation (Transformation|GetWorldLocation _widget) (Transformation|GetWorldLocation (Variables|/Game/Blueprints/Player/BP_ThirdPersonCharacter.BP_ThirdPersonCharacter_C|GetFollowCamera (.AsBP%20Third%20Person%20Character (Utilities|Casting|CastToBP_ThirdPersonCharacter (Game|GetPlayerCharacter 0)))))) false false))

(event EventTakeDamage
  (params (damages :type Integer))
  (bind _maxhealth (Variables|Default|GetmaxHealth))
  (bind _output_get (Variables|Default|Sethealth (Math|Integer|Clamp(Integer) (- (Variables|Default|Gethealth) damages) 0 _maxhealth)))
  (Variables|/Script/UMG.ProgressBar|SetPercent (Variables|/Game/Carl/WB_EnemyHealthBar.WB_EnemyHealthBar_C|GethealthBar (.AsWB%20Enemy%20Health%20Bar (Utilities|Casting|CastToWB_EnemyHealthBar (UserInterface|GetWidget (Variables|Default|GetWidget))))) (/ (Math|Conversions|ToFloat(Integer) _output_get) (Math|Conversions|ToFloat(Integer) _maxhealth)))
  (if (<= (Math|Integer|Clamp(Integer) (- (Variables|Default|Gethealth) damages) 0 _maxhealth) 0)
    (CallFunction|Die)))

(event EventDie
  (for _index (range 0 (Variables|Default|GetberriesAmount))
    (Game|SpawnActorfromClass "/Game/Blueprints/Berries/BP_Berry.BP_Berry_C" (Math|Transform|MakeTransform (+ (Transformation|GetActorLocation) "0.000000,0.000000,1000.000000")) "Undefined" "MultiplyWithRoot" 0 0))
  (Actor|DestroyActor))

(event EventMeleeAttack
  (params (targetToAttack :type Actor%20Object%20Reference))
  (bind _ac_finishattackanimation (Variables|Default|GetAC_FinishAttackAnimation))
  (Utilities|IsValid targetToAttack
    (:Is%20Valid
      (Variables|Default|SetisAttacking true)
      (Class|BPIDamagable|TakeDamage(Message) targetToAttack (Variables|Default|Getdamages))
      (Utilities|FlowControl|Delay 1.5)
      (Class|BPIEvent|Notify(Message) _ac_finishattackanimation))
    (:Is%20Not%20Valid
      (Default|Notify _ac_finishattackanimation))))

(fn ConstructionScript)

(fn End&attack
  (Class|BPIEvent|Notify(Message) (Variables|Default|GetAC_FinishAttackAnimation)))

(fn GetIsDead
  (return false))