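; BP_Door is a double door that opens for a player character holding a key.
; A sphere overlap casts the other actor to BP_ThirdPersonCharacter and checks HasKey, printing "Game Over" when the key is missing.
; With the key, the Open event plays a timeline that yaws the left and right door meshes in opposite directions.
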(event OnComponentBeginOverlap(Sphere)
  (params (OverlappedComponent :type Primitive%20Component%20Object%20Reference) (OtherActor :type Actor%20Object%20Reference) (OtherComp :type Primitive%20Component%20Object%20Reference) (OtherBodyIndex :type Integer) (bFromSweep :type Boolean) (SweepResult :type Hit%20Result%20Structure%20%28by%20ref%29))
  (bind _asbp_third_person_character (Utilities|Casting|CastToBP_ThirdPersonCharacter OtherActor))
  (if (Variables|/Game/Blueprints/Player/BP_ThirdPersonCharacter.BP_ThirdPersonCharacter_C|GethasKey _asbp_third_person_character)
    (CallFunction|Open)
    (else
      (Development|PrintString "Game Over"))))

(event Custom|Open
  (bind _rotation (Timeline|Timeline Play)
    (:Update
      (Transformation|SetRelativeRotation (Variables|Default|GetSM_LeftDoor_04) (Math|Rotator|MakeRotator 0.0 0.0 _rotation) false false)
      (Transformation|SetRelativeRotation (Variables|Default|GetSM_RightDoor_04) (Math|Rotator|MakeRotator 0.0 0.0 (* _rotation -1.0)) false false))))

(event EventBeginPlay)

(event Collision|EventActorBeginOverlap
  (params (OtherActor :type Actor%20Object%20Reference)))

(event EventTick
  (params (DeltaSeconds :type Float%20%28single-precision%29)))

(fn ConstructionScript)